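; BPC_Door is a door component that gates opening behind a matching key ID.
; InteractedWith compares the supplied key ID to the component's KeyID and branches to success or failure.
; On success it prints a debug message, casts its owner to BP_DoorObject and calls Open on it.
; On failure it only prints a debug message.
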(event `InteractedWith`
  (params (CurrentKeyID :type Integer))
  ;[1 0 0.8671 0.5] Check Key is Valid
  (if (== (`self.KeyID`) CurrentKeyID)
    (`self.OpenDoor`)
    (else
      (`self.FailToOpenDoor`))))

(event `OpenDoor`
  (bind _returnvalue (`self.GetOwner`))
  ;[0.2812 0.9391 0 0.5] Key is Valid
  (`KismetSystemLibrary.PrintString` "SUCCESSFULLY OPENED DOOR")
  (`/Engine/EditorBlueprintResources/StandardMacros.IsValid` _returnvalue
    (:`Is Valid`
      (bind _asbp_door_object (cast `/Game/BP_DoorObject` _returnvalue))
      (`/Game/BP_DoorObject.Open` _asbp_door_object))))

(event `FailToOpenDoor`
  ;[1 0.00619 0.003584 0.5] Key Not Valid
  (`KismetSystemLibrary.PrintString` "FAILED TO OPEN DOOR"))