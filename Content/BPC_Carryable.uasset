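; Actor component that lets its owning actor be picked up, carried in front of the player camera, and dropped.
; PickedUp disables collision, flags InHand, attaches the owner to the camera and sets its relative location to the hand offset, printing debug success or failure.
; Dropped detaches it, restores collision, moves it to the drop point, then line-traces downward to rest it slightly above the surface hit.
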(event `PickedUp`
  (params (PlayerCamera :type "CameraComponent Object Reference") (PlayerHand :type "Vector Structure"))
  (bind _returnvalue (`self.GetOwner`))
  (`Actor.SetActorEnableCollision` _returnvalue false)
  (set `self.InHand?` true)
  (`/Engine/EditorBlueprintResources/StandardMacros.IsValid` PlayerCamera
    (:`Is Valid`
      (bind _returnvalue_2 (`Actor.K2_AttachToComponent` _returnvalue PlayerCamera "None" "KeepRelative" "KeepRelative" "KeepRelative" true))
      (if _returnvalue_2
        (`KismetSystemLibrary.PrintString` "attach success")
        (`Actor.K2_SetActorRelativeLocation` _returnvalue PlayerHand false false)
        (else
          (`KismetSystemLibrary.PrintString` "NO ATTACH NO"))))))

(event `Dropped`
  (params (LocationToDrop :type "Vector Structure"))
  (bind _returnvalue (`self.GetOwner`))
  (bind (_returnvalue_x _returnvalue_y _returnvalue_z) (`KismetMathLibrary.BreakVector` (`Actor.K2_GetActorLocation` _returnvalue)))
  (`Actor.K2_DetachFromActor` _returnvalue "KeepRelative" "KeepRelative" "KeepRelative")
  (set `self.InHand?` false)
  (`Actor.SetActorEnableCollision` _returnvalue true)
  (`Actor.K2_SetActorLocation` _returnvalue LocationToDrop false false)
  (bind (_outhit _returnvalue_2) (`KismetSystemLibrary.LineTraceSingle` (`KismetMathLibrary.MakeVector` _returnvalue_x _returnvalue_y _returnvalue_z) (`KismetMathLibrary.MakeVector` _returnvalue_x _returnvalue_y (- _returnvalue_z 1000.0)) "TraceTypeQuery1"))
  (if _returnvalue_2
    (bind (_bblockinghit _binitialoverlap _time _distance _location _impactpoint) (`GameplayStatics.BreakHitResult` _outhit))
    (`Actor.K2_SetActorLocation` _returnvalue (`KismetMathLibrary.MakeVector` (.x _impactpoint) (.y _impactpoint) (+ (.z _impactpoint) 15.0)) false false)))