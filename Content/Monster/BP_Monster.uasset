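; BP_Monster is a monster that advances along the X axis on a looping timer, at a speed set by the nearest slowdown light.
; Each step scales with the initial X distance to its End component, using a separate speed multiplier when the current light is inactive.
; When its hitbox overlaps that light, it drops it from the list and targets the nearest remaining one.
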(event `self.ReceiveBeginPlay`
  (bind _returnvalue_x (`KismetMathLibrary.BreakVector` (`self.K2_GetActorLocation`)))
  (bind _returnvalue_x_2 (`KismetMathLibrary.BreakVector` (`SceneComponent.K2_GetComponentLocation` (`self.End`))))
  ; BeginPlay
  (`|ExecutionSequence`
    (:`then_0`
      (bind _outactors (`GameplayStatics.GetAllActorsOfClass` "/Game/Lights/BP_SlowdownLight.BP_SlowdownLight_C"))
      (bind _output_get (set `self.Lights` _outactors))
      (set `self.CurrentLight` (`.ReturnValue` (`GameplayStatics.FindNearestActor` (`self.K2_GetActorLocation`) _output_get))))
    (:`then_1`
      (set `self.TotalDistance` (- _returnvalue_x_2 _returnvalue_x))
      (`KismetSystemLibrary.K2_SetTimerDelegate` (`|CreateDelegate` :!event `ProgressMonster`) (`self.TimeBetweenUpdates`) true))))

(event `ProgressMonster`
  (bind (_returnvalue_x _returnvalue_y _returnvalue_z) (`KismetMathLibrary.BreakVector` (`self.K2_GetActorLocation`)))
  ;[0 0.07618 0.15 0.5] Event to move monster
  (bind _active (message `/Game/Lights/BPI_SlowdownLight.GetActive` (`self.CurrentLight`)))
  (if _active
    (set `self.SpeedMultiplier` 1.0)
    (else
      (set `self.SpeedMultiplier` (`self.InDarkSpeedMultiplier`))))
  (`self.K2_SetActorLocation` (`KismetMathLibrary.MakeVector` (+ (* (`self.TotalDistance`) (`self.TimeBetweenUpdates`) (* (`self.BaseSpeed`) (`self.SpeedMultiplier`))) _returnvalue_x) _returnvalue_y _returnvalue_z)))

(event `self.Hitbox.OnComponentBeginOverlap`
  (params (OverlappedComponent :type "PrimitiveComponent Object Reference") (OtherActor :type "Actor Object Reference") (OtherComp :type "PrimitiveComponent Object Reference") (OtherBodyIndex :type Integer) (bFromSweep :type Boolean) (SweepResult :type "HitResult Structure (by ref)"))
  ;[0.6875 0 0.01095 0.5] HitboxBeginOverlap
  (if (== OtherActor (`self.CurrentLight`))
    (`KismetArrayLibrary.Array_RemoveItem` (`self.Lights`) (`self.CurrentLight`))
    (set `self.CurrentLight` (`.ReturnValue` (`GameplayStatics.FindNearestActor` (`self.K2_GetActorLocation`) (`self.Lights`))))))

(fn `UserConstructionScript`)