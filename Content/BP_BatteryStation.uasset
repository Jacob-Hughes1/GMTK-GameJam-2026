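; Interactable battery station that takes batteries from the player and charges over time to open an exit door.
; Interacting with a held item that has a battery component removes it through the initiator, increments the battery count and steps up the charge rate.
; Tick accumulates charge from rate times battery count, printing the value, then opens the linked door once when full.
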(event `self.ReceiveTick`
  (params (DeltaSeconds :type "Float (single-precision)"))
  (bind _exitdoor (`self.ExitDoor`))
  ;[1 0 0.8671 0.5] Battery Charging
  (if (`self.doorOpen?`)
    _
    (elif (> (`self.BatteryCount`) 0)
      (set `self.Delta Seconds` DeltaSeconds)
      (if (< (`self.CurrentCharge`) 100.0)
        (bind _output_get (set `self.CurrentCharge` (+ (`self.CurrentCharge`) (* (* (`self.Delta Seconds`) (`self.BatteryChargeRate`)) (`self.BatteryCount`)))))
        (`KismetSystemLibrary.PrintString` (`KismetStringLibrary.Conv_DoubleToString` _output_get))
        (else
          (`/Engine/EditorBlueprintResources/StandardMacros.DoOnce` false
            (:`Completed`
              (set `self.doorOpen?` true)
              (`/Engine/EditorBlueprintResources/StandardMacros.IsValid` _exitdoor
                (:`Is Valid`
                  (`/Game/BP_ExitDoor.Open` _exitdoor))))))))))

(event `/Game/FirstPerson/Blueprints/BPI_Interact.Interact`
  (params (Initiator :type "Actor Object Reference (by ref)") (HeldItem :type "Actor Object Reference (by ref)"))
  (`/Engine/EditorBlueprintResources/StandardMacros.IsValid` HeldItem
    (:`Is Valid`
      (`/Engine/EditorBlueprintResources/StandardMacros.IsValid` (`self.GetComponentByClass` HeldItem "/Game/Items/BPC_Battery.BPC_Battery_C")
        (:`Is Valid`
          (message `/Game/FirstPerson/Blueprints/BPI_PlayerInterface.DestroyHand` Initiator)
          (bind _output_get (set `self.BatteryCount` (+ (`self.BatteryCount`) 1)))
          (switch `int` (- _output_get 1)
            (:`0`
              (set `self.BatteryChargeRate` 0.5))
            (:`1`
              (set `self.BatteryChargeRate` 1.0))
            (:`2`
              (set `self.BatteryChargeRate` 2.0))))))))

(fn `GetText`
  (returns (TextOutput :type Text))
  (return "Bring Battery To Charge"))

(fn `UserConstructionScript`)