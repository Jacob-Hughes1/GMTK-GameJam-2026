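; BP_SlowdownLight is an interactable lantern with a depletable charge that dims as it runs out.
; Looping timers adjust the clamped charge, with depletion meant to run from BeginPlay and recharging started by Interact, which never stops it.
; Each change scales the point light from its starting intensity and updates an Active flag, exposed through GetActive, that turns false at zero charge.
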(event `self.ReceiveBeginPlay`
  ; BeginPlay
  (`|ExecutionSequence`
    (:`then_0`
      (set `self.Charge` (`self.MaxCharge`))
      (set `self.MaxIntensity` (`LightComponentBase.Intensity` (`self.PointLight`))))
    (:`then_1`
      (`KismetSystemLibrary.K2_SetTimerDelegate` (`|CreateDelegate` :!event `DepleteCharge`) (`self.UpdateTimer`) true))))

(event `DepleteCharge`
  ;[0.5469 0 0.007708 0.5] Event to reduce lantern charge from timer
  (set `self.Charge` (`KismetMathLibrary.FClamp` (- (`self.Charge`) (* (`self.DepletionRate`) (`self.UpdateTimer`))) 0.0 (`self.MaxCharge`)))
  (`self.OnChargeChanged`))

(event `/Game/FirstPerson/Blueprints/BPI_Interact.Interact`
  (params (Initiator :type "Actor Object Reference (by ref)") (HeldItem :type "Actor Object Reference (by ref)"))
  (`KismetSystemLibrary.K2_SetTimerDelegate` (delegate `ChargeLantern`) (`self.UpdateTimer`) true))

(event `ChargeLantern`
  ;[0.07695 0.5104 0 0.5] Event to increase lantern charge from timer
  (set `self.Charge` (`KismetMathLibrary.FClamp` (+ (`self.Charge`) (* (`self.ChargeRate`) (`self.UpdateTimer`))) 0.0 (`self.MaxCharge`)))
  (`self.OnChargeChanged`))

(fn `GetActive`
  (returns (Active :type Boolean))
  (return (`self.Active`)))

(fn `OnChargeChanged`
  (`LightComponent.SetIntensity` (`self.PointLight`) (* (/ (`self.Charge`) (`self.MaxCharge`)) (`self.MaxIntensity`)))
  (if (<= (`self.Charge`) 0.0)
    (set `self.Active` false)
    (else
      (set `self.Active` true))))

(fn `UserConstructionScript`)